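; BP_Weapon_Kalash is a child weapon Blueprint for the player's Kalash assault rifle, supplying its shoot, reload and zoom presentation on top of the parent class.
; It snaps to the character's normal socket on BeginPlay, then moves between that and the zoom socket when aiming, toggling the crosshair.
; Shooting and reloading play mesh animations with camera shake or widget feedback, while a DoOnce limits the aim sound to once per zoom-in.
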(event EventFChildPlayerZoom
  (params (ZoomIn? :type Boolean))
  (bind _as_bp_character (Variables|Default|GetAs%20BP%20Character))
  ;[0.3495 0.3811 0.6146] Zoom
  (if ZoomIn?
    (Transformation|AttachComponentToComponent (Variables|/Game/Blueprints/Character/BP_Character.BP_Character_C|GetKalashZoomSocket _as_bp_character) "None" "KeepRelative" "KeepRelative" "KeepRelative" true)
    (CallFunction|FCrossHairVisibility "Hidden")
    (Utilities|FlowControl|DoOnce false :!label _label
      (:Completed
        (Audio|PlaySound2D "/Game/MilitaryWeapSilver/Sound/Pistol/Aim.Aim" 9.0 1.0 0.0 0 0)))
    (else
      (Transformation|AttachComponentToComponent (Variables|/Game/Blueprints/Character/BP_Character.BP_Character_C|GetKalashNormalSocket _as_bp_character) "None" "KeepRelative" "KeepRelative" "KeepRelative" true)
      (CallFunction|FCrossHairVisibility "Visible")
      (goto _label Reset))))

(event EventFChildPlayerShoot
  ;[0.2776 0.9303 1] Shoot
  (Components|Animation|PlayAnimation (Variables|Default|GetAssault) "/Game/MilitaryWeapSilver/Weapons/Animations/Fire_Rifle_W.Fire_Rifle_W" false)
  (Game|Feedback|ClientStartCameraShake (Game|GetPlayerController 0) "/Game/Blueprints/Character/CameraShake/BP_CameraShake_Shoot.BP_CameraShake_Shoot_C" 1.0 "CameraLocal" "0, 0, 0"))

(event EventBeginPlay
  ;[1 0.2292 0.2292] Begin Play
  (|CallParentFunction)
  (Transformation|AttachComponentToComponent (Variables|/Game/Blueprints/Character/BP_Character.BP_Character_C|GetKalashNormalSocket (Variables|Default|GetAs%20BP%20Character)) "None" "SnapToTarget" "SnapToTarget" "SnapToTarget" true))

(event EventFChildPlayerReload
  ;[0.1302 1 0.03963] Reload
  (Components|Animation|PlayAnimation (Variables|Default|GetAssault) "/Game/MilitaryWeapSilver/Weapons/Animations/Prone_Reload_Rifle_W.Prone_Reload_Rifle_W" false)
  (Default|ReloadAnimation (Variables|Default|GetUW_Weapon_Reference) false))

(fn ConstructionScript
  (|CallParentFunction))