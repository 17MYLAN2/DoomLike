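; Player pistol component handling aiming, shooting, reloading and ammo, with a UW_Weapon HUD widget created at BeginPlay.
; Aiming snaps the pistol between the character's zoom and normal sockets and toggles the crosshair.
; Shots line-trace from the camera and message BPI_Weapon actors, with animation, camera shake and low-ammo warnings.
; Delayed reloads always fill the magazine, clamping the reserve at zero, and AddMaxAmmo tops up that reserve.
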(event Input|EnhancedActionEvents|EnhancedInputActionIA_Shoot
  (params (ActionValue :type Boolean) (ElapsedSeconds :type Float%20%28double-precision%29) (TriggeredSeconds :type Float%20%28double-precision%29) (InputAction :type Input%20Action%20Object%20Reference :default "/Game/Blueprints/Character/Inputs/IA_Shoot.IA_Shoot"))
  ;[0.06829 0.2708 0] Shoot System
  (if (and (Variables|Default|GetCanShoot?) (not (Variables|Default|GetIsReloading?)))
    (Utilities|FlowControl|Sequence
      (:then_0
        (Math|Integer|DecrementInt (Variables|Default|GetCurrentAmmo)
          (:%20%20
            (CallFunction|ShootSystem)
            (CallFunction|CheckifEnoughAmmo))))
      (:then_1
        (Default|UpdateAmmoText (Variables|Default|GetUW_Weapon) (Variables|Default|GetCurrentAmmo) (Variables|Default|GetMaxAmmo)))
      (:then_2
        (Components|Animation|PlayAnimation (Variables|/Game/Blueprints/Character/BP_Character.BP_Character_C|GetPistols_A (Variables|Default|GetAs%20BP%20Character)) "/Game/MilitaryWeapSilver/Weapons/Animations/Fire_Pistol_W.Fire_Pistol_W" false)
        (Game|Feedback|ClientStartCameraShake (Game|GetPlayerController 0) "/Game/Blueprints/Character/CameraShake/BP_CameraShake_Shoot.BP_CameraShake_Shoot_C" 1.0 "CameraLocal" "0, 0, 0")))
    (else
      (Audio|PlaySound2D "/Game/MilitaryWeapSilver/Sound/Pistol/EmptyGun.EmptyGun" 1.0 1.0 0.0 0 0))))

(event Input|EnhancedActionEvents|EnhancedInputActionIA_Reload
  (params (ActionValue :type Boolean) (ElapsedSeconds :type Float%20%28double-precision%29) (TriggeredSeconds :type Float%20%28double-precision%29) (InputAction :type Input%20Action%20Object%20Reference :default "/Game/Blueprints/Character/Inputs/IA_Reload.IA_Reload"))
  ;[0 1 0.68] Reload System
  (if (Math|Boolean|ANDBoolean (< (Variables|Default|GetCurrentAmmo) (Variables|Default|GetMaxAmmoOnMag)) (> (Variables|Default|GetMaxAmmo) 0) (not (Variables|Default|GetIsReloading?)))
    (Utilities|FlowControl|Sequence
      (:then_0
        (Variables|Default|SetIsReloading? true))
      (:then_1
        (Components|Animation|PlayAnimation (Variables|/Game/Blueprints/Character/BP_Character.BP_Character_C|GetPistols_A (Variables|Default|GetAs%20BP%20Character)) "/Game/MilitaryWeapSilver/Weapons/Animations/Reload_Pistol_W.Reload_Pistol_W" false))
      (:then_2
        (Utilities|FlowControl|Delay (Variables|Default|GetReloadDuration))
        (CallFunction|ReloadCalcul)))))

(event Input|EnhancedActionEvents|EnhancedInputActionIA_GunZoom
  (params (ActionValue :type Vector%202D%20Structure) (ElapsedSeconds :type Float%20%28double-precision%29) (TriggeredSeconds :type Float%20%28double-precision%29) (InputAction :type Input%20Action%20Object%20Reference :default "/Game/Blueprints/Character/Inputs/IA_GunZoom.IA_GunZoom"))
  (bind _as_bp_character (Variables|Default|GetAs%20BP%20Character))
  (bind _pistols_a (Variables|/Game/Blueprints/Character/BP_Character.BP_Character_C|GetPistols_A _as_bp_character))
  ;[1 0.3058 0.2361] Aim System
  (:Ongoing
    (Transformation|AttachComponentToComponent _pistols_a (Variables|/Game/Blueprints/Character/BP_Character.BP_Character_C|GetZoomSocket _as_bp_character) "None" "SnapToTarget" "SnapToTarget" "SnapToTarget" true)
    (CallFunction|CrossHairVisibility "Hidden"))
  (:Canceled
    (Transformation|AttachComponentToComponent _pistols_a (Variables|/Game/Blueprints/Character/BP_Character.BP_Character_C|GetNormalSocket _as_bp_character) "None" "SnapToTarget" "SnapToTarget" "SnapToTarget" true :!label _label)
    (CallFunction|CrossHairVisibility "Visible"))
  (:Completed
    (goto _label)))

(event EventBeginPlay
  ;[1 0.07451 0.07451] Begin Play
  (Utilities|FlowControl|Sequence
    (:then_0
      ;;[0 1 0.2742] Create BP_Character Reference
      (bind _asbp_character (Utilities|Casting|CastToBP_Character (Game|GetPlayerCharacter 0)))
      (Variables|Default|SetAs%20BP%20Character _asbp_character))
    (:then_1
      ;;[1 0.3042 0] Create UW_Weapon Reference
      (bind _returnvalue (UserInterface|CreateWidget "/Game/Widgets/Weapon/UW_Weapon.UW_Weapon_C"))
      (bind _output_get (Variables|Default|SetUW_Weapon _returnvalue))
      (UserInterface|Viewport|AddtoViewport _output_get 0))
    (:then_2
      ;;[0 1 0.1329] Initialize Weapon Options
      (CallFunction|InitializeWeaponOptions))))

(fn InitializeWeaponOptions
  (bind _uw_weapon (Variables|Default|GetUW_Weapon))
  (bind _output_get (Variables|Default|SetCurrentAmmo (Variables|Default|GetMaxAmmoOnMag)))
  (Default|UpdateAmmoText _uw_weapon _output_get (Variables|Default|GetMaxAmmo))
  (Widget|SetVisibility (Variables|/Game/Widgets/Weapon/UW_Weapon.UW_Weapon_C|GetLowAmmo _uw_weapon) "Hidden")
  (Default|ReloadAnimation (Variables|Default|GetUW_Weapon) false)
  (Variables|Default|SetIsReloading? false)
  (Variables|Default|SetCanShoot? true))

(fn CheckifEnoughAmmo
  (if (<= (Variables|Default|GetCurrentAmmo) 4)
    (Widget|SetVisibility (Variables|/Game/Widgets/Weapon/UW_Weapon.UW_Weapon_C|GetLowAmmo (Variables|Default|GetUW_Weapon)) "Visible")
    (Default|ReloadAnimation (Variables|Default|GetUW_Weapon) true))
  (if (<= (Variables|Default|GetCurrentAmmo) 0)
    (Variables|Default|SetCanShoot? false)))

(fn ShootSystem
  (bind _as_bp_character (Variables|Default|GetAs%20BP%20Character))
  (bind _camera (Variables|/Game/Blueprints/Character/BP_Character.BP_Character_C|GetCamera _as_bp_character))
  (bind _returnvalue (Transformation|GetWorldLocation _camera))
  (bind (_outhit _returnvalue_2) (Collision|LineTraceByChannel _returnvalue (+ _returnvalue (* (Math|Vector|GetForwardVector _camera) (Variables|Default|GetShootingDistance))) "TraceTypeQuery1" false 0 "ForDuration" true "(R=1.000000,G=0.000000,B=0.000000,A=1.000000)" "(R=0.000000,G=1.000000,B=0.000000,A=1.000000)" 0.2))
  (if (and _returnvalue_2 (Utilities|DoesObjectImplementInterface (.HitActor (Collision|BreakHitResult _outhit)) "/Game/Blueprints/Interfaces/BPI_Weapon.BPI_Weapon_C"))
    (Class|BPIWeapon|ActorHit(Message) (.HitActor (Collision|BreakHitResult _outhit)))))

(fn CrossHairVisibility
  (params (InVisibility :type ESlateVisibility%20Enum :default "Visible"))
  (Widget|SetVisibility (Variables|/Game/Widgets/Main/UW_Main.UW_Main_C|GetCrossHair (Variables|/Game/Blueprints/Character/BP_Character.BP_Character_C|GetUW_Main (Variables|Default|GetAs%20BP%20Character))) InVisibility))

(fn ReloadCalcul
  (Variables|Default|SetMissingBulletOnMag (- (Variables|Default|GetMaxAmmoOnMag) (Variables|Default|GetCurrentAmmo)))
  (Variables|Default|SetMaxAmmo (- (Variables|Default|GetMaxAmmo) (Variables|Default|GetMissingBulletOnMag)))
  (Variables|Default|SetCurrentAmmo (Variables|Default|GetMaxAmmoOnMag))
  (if (< (Variables|Default|GetMaxAmmo) 0)
    (Variables|Default|SetMaxAmmo 0))
  (Default|UpdateAmmoText (Variables|Default|GetUW_Weapon) (Variables|Default|GetCurrentAmmo) (Variables|Default|GetMaxAmmo))
  (Variables|Default|SetCanShoot? true)
  (Variables|Default|SetIsReloading? false))

(fn AddMaxAmmo
  (params (AmmoToAdd :type Integer))
  (bind _output_get (Variables|Default|SetMaxAmmo (+ AmmoToAdd (Variables|Default|GetMaxAmmo))))
  (Default|UpdateAmmoText (Variables|Default|GetUW_Weapon) (Variables|Default|GetCurrentAmmo) _output_get))