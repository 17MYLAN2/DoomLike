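; Base weapon Blueprint that attaches to the player character and handles shooting, reloading, zoom and ammo.
; Empty child events let subclasses add shoot, zoom and reload behavior.
; A camera line trace messages BPI_Weapon actors or spawns a bullet impact, running even when firing is blocked.
; Ammo changes update its widget, which flags low ammo; a delayed reload always fills the magazine, clamping reserves at zero.
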(event Custom|F_PlayerShoot
  ;[1 0.1647 0.1961] Events - Shoot
  (CallFunction|FShootSystem)
  (CallFunction|FShootDistance))

(event Custom|F_ChildPlayerShoot
  ;[1 0.1647 0.1961] Events - Shoot
)

(event Custom|F_PlayerZoom
  (params (ZoomIn? :type Boolean))
  ;[1 0.1647 0.1961] Event - Zoom
  (CallFunction|FChildPlayerZoom ZoomIn?))

(event Custom|F_ChildPlayerZoom
  (params (ZoomIn? :type Boolean))
  ;[1 0.1647 0.1961] Event - Zoom
)

(event Custom|F_PlayerReload
  ;[1 0.1647 0.1961] Event - Reload
  (if (Math|Boolean|ANDBoolean (< (Variables|Default|GetCurrentAmmo) (Variables|Default|GetMaxAmmoOnMag)) (> (Variables|Default|GetMaxAmmo) 0) (not (Variables|Default|GetIsReloading?)))
    (Variables|Default|SetIsReloading? true)
    (CallFunction|FChildPlayerReload)
    (Utilities|FlowControl|Delay 2.0)
    (CallFunction|FReloadCalcul)))

(event Custom|F_ChildPlayerReload
  ;[1 0.1647 0.1961] Event - Reload
)

(event EventBeginPlay
  ;[1 0.1647 0.1961] Begin Play
  (Utilities|FlowControl|Sequence
    (:then_0
      ;;[0.3571 0.7109 1] Create Reference to BP_Character
      (bind _asbp_character (Utilities|Casting|CastToBP_Character (Game|GetPlayerCharacter 0)))
      (Variables|Default|SetAs%20BP%20Character _asbp_character)
      (Variables|/Game/Blueprints/Character/BP_Character.BP_Character_C|SetWeaponRef _asbp_character self))
    (:then_1
      ;;[0.5172 1 0.1739] Create Widget
      (bind _returnvalue (UserInterface|CreateWidget "/Game/Widgets/Weapon/UW_Weapon.UW_Weapon_C"))
      (bind _output_get (Variables|Default|SetUW_Weapon_Reference _returnvalue))
      (UserInterface|Viewport|AddtoViewport _output_get 0))
    (:then_2
      (Transformation|AttachComponentToComponent (Variables|/Game/Blueprints/Character/BP_Character.BP_Character_C|GetNormalSocket (Variables|Default|GetAs%20BP%20Character)) "None" "SnapToTarget" "SnapToTarget" "SnapToTarget" true)
      (CallFunction|FInitializeWeapon))))

(fn ConstructionScript)

(fn FShootDistance
  (bind _as_bp_character (Variables|Default|GetAs%20BP%20Character))
  (bind _camera (Variables|/Game/Blueprints/Character/BP_Character.BP_Character_C|GetCamera _as_bp_character))
  (bind _returnvalue (Transformation|GetWorldLocation _camera))
  (bind (_outhit _returnvalue_2) (Collision|LineTraceByChannel _returnvalue (+ _returnvalue (* (Math|Vector|GetForwardVector _camera) (Variables|Default|GetShootDistance))) "TraceTypeQuery1" false 0 "None" true "(R=1.000000,G=0.000000,B=0.000000,A=1.000000)" "(R=0.000000,G=1.000000,B=0.000000,A=1.000000)" 0.2))
  (if (and _returnvalue_2 (Utilities|DoesObjectImplementInterface (.HitActor (Collision|BreakHitResult _outhit)) "/Game/Blueprints/Interfaces/BPI_Weapon.BPI_Weapon_C"))
    (Class|BPIWeapon|ActorHit(Message) (.HitActor (Collision|BreakHitResult _outhit)))
    (else
      (Game|SpawnActorfromClass "/Game/Blueprints/Weapon/BP_BulletImpact.BP_BulletImpact_C" (Math|Conversions|ToTransform(Vector) (.ImpactPoint (Collision|BreakHitResult _outhit))) "Undefined" "MultiplyWithRoot" 0 0))))

(fn FShootSystem
  (if (and (Variables|Default|GetCanShoot?) (not (Variables|Default|GetIsReloading?)))
    (Math|Integer|DecrementInt (Variables|Default|GetCurrentAmmo)
      (:%20%20
        (CallFunction|FChildPlayerShoot)
        (CallFunction|FCheckifEnoughAmmo)
        (Default|UpdateAmmoText (Variables|Default|GetUW_Weapon_Reference) (Variables|Default|GetCurrentAmmo) (Variables|Default|GetMaxAmmo))))
    (else
      (Audio|PlaySound2D "/Game/MilitaryWeapSilver/Sound/Pistol/EmptyGun.EmptyGun" 1.0 1.0 0.0 0 0))))

(fn FCheckifEnoughAmmo
  (if (<= (Variables|Default|GetCurrentAmmo) 4)
    (Default|ReloadAnimation (Variables|Default|GetUW_Weapon_Reference) true))
  (if (<= (Variables|Default|GetCurrentAmmo) 0)
    (Variables|Default|SetCanShoot? false)))

(fn FInitializeWeapon
  (bind _uw_weapon_reference (Variables|Default|GetUW_Weapon_Reference))
  (bind _output_get (Variables|Default|SetCurrentAmmo (Variables|Default|GetMaxAmmoOnMag)))
  (Default|UpdateAmmoText _uw_weapon_reference _output_get (Variables|Default|GetMaxAmmo))
  (Widget|SetVisibility (Variables|/Game/Widgets/Weapon/UW_Weapon.UW_Weapon_C|GetLowAmmo _uw_weapon_reference) "Hidden")
  (Default|ReloadAnimation _uw_weapon_reference false)
  (Variables|Default|SetIsReloading? false)
  (Variables|Default|SetCanShoot? true))

(fn FCrossHairVisibility
  (params (InVisibility :type ESlateVisibility%20Enum :default "Visible"))
  (Widget|SetVisibility (Variables|/Game/Widgets/Main/UW_Main.UW_Main_C|GetCrossHair (Variables|/Game/Blueprints/Character/BP_Character.BP_Character_C|GetUW_Main (Variables|Default|GetAs%20BP%20Character))) InVisibility))

(fn FReloadCalcul
  (Variables|Default|SetMissingBulletOnMag (- (Variables|Default|GetMaxAmmoOnMag) (Variables|Default|GetCurrentAmmo)))
  (Variables|Default|SetMaxAmmo (- (Variables|Default|GetMaxAmmo) (Variables|Default|GetMissingBulletOnMag)))
  (Variables|Default|SetCurrentAmmo (Variables|Default|GetMaxAmmoOnMag))
  (if (< (Variables|Default|GetMaxAmmo) 0)
    (Variables|Default|SetMaxAmmo 0))
  (Default|UpdateAmmoText (Variables|Default|GetUW_Weapon_Reference) (Variables|Default|GetCurrentAmmo) (Variables|Default|GetMaxAmmo))
  (Variables|Default|SetCanShoot? true)
  (Variables|Default|SetIsReloading? false))

(fn FAddMaxAmmo
  (params (AmmoNumber :type Integer))
  (Variables|Default|SetMaxAmmo (+ (Variables|Default|GetMaxAmmo) AmmoNumber))
  (Default|UpdateAmmoText (Variables|Default|GetUW_Weapon_Reference) (Variables|Default|GetCurrentAmmo) (Variables|Default|GetMaxAmmo)))